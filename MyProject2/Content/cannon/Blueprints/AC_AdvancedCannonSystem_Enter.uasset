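; Actor component that lets the player approach and take control of an advanced cannon pawn.
; Display_text shows an enter prompt widget when near a cannon and removes it otherwise.
; Enter_vehicle, when use and proximity flags are set, stores the player character on the cannon, possesses it, hides and disables collision on the character, then removes the prompt.
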(event `Display_text`
  ;[1 0.09237 0.9718] Display enter text
  (if (`self.bNear_BP_AdvancedCannonSystem_?`)
    (bind _returnvalue (`|CreateWidget` "/Game/cannon/Blueprints/WBP_AdvancedCannonSystem_enter.WBP_AdvancedCannonSystem_enter_C" (`GameplayStatics.GetPlayerController` 0)))
    (`UserWidget.AddToViewport` _returnvalue 0)
    (else
      (`/Engine/EditorBlueprintResources/StandardMacros.IsValid` _returnvalue
        (:`Is Valid`
          (`Widget.RemoveFromParent` _returnvalue :!label _label))))))

(event `Enter_vehicle`
  (bind _bp_advancedcannonsystem (`self.BP_AdvancedCannonSystem`))
  ;[1 0.02277 0.904] Posses vehicle
  (if (and (`self.bUse_BP_AdvancedCannonSystem`) (`self.bNear_BP_AdvancedCannonSystem_?`))
    (set `/Game/cannon/Blueprints/BP_AdvancedCannonSystem.Use_AdvancedCannonSystem` true _bp_advancedcannonsystem)
    (bind _output_get (set `/Game/cannon/Blueprints/BP_AdvancedCannonSystem.Character` (`GameplayStatics.GetPlayerCharacter` 0) _bp_advancedcannonsystem))
    (`Controller.Possess` (`GameplayStatics.GetPlayerController` 0) _bp_advancedcannonsystem)
    (`Actor.SetActorHiddenInGame` _output_get true)
    (`Actor.SetActorEnableCollision` _output_get false)
    (goto _label)))