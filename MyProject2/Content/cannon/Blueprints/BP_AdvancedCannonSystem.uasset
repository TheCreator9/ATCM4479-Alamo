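; Possessable stationary cannon that the player enters through a trigger and enter component, with a HUD, and leaves by repossessing their character.
; Look input aims turret and barrel, right mouse zooms the first- or third-person camera, and F toggles slow motion.
; Firing spawns projectiles from a shell count that a timeline can replenish, with an optional timer-driven auto-fire mode.
; Optionally, Tick rebuilds a spline-mesh trajectory preview from predicted projectile paths.
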(event `CE_Auto_Fire`
  (bind _the_barrel_of_the_cannon_staticmesh_2 (`self.The_barrel_of_the_cannon_StaticMesh_2`))
  (bind _returnvalue (`SceneComponent.GetSocketLocation` _the_barrel_of_the_cannon_staticmesh_2 "None"))
  ;[0.233 0.09733 0.2471] Nodes auto fire projectile destination
  (if (`self.Use_Auto_Fire`)
    (`KismetSystemLibrary.LineTraceSingle` _returnvalue (+ _returnvalue (* (`KismetMathLibrary.Conv_RotatorToVector` (`SceneComponent.GetSocketRotation` _the_barrel_of_the_cannon_staticmesh_2 "None")) 50000.0)) "TraceTypeQuery1")))

(event `EnhancedInput|/Game/cannon/Demo/EpicContent/Input/Actions/IA_Fire`
  (params (ActionValue :type "Vector2D Structure") (ElapsedSeconds :type "Float (double-precision)") (TriggeredSeconds :type "Float (double-precision)") (InputAction :type "InputAction Object Reference" :default "/Game/cannon/Demo/EpicContent/Input/Actions/IA_Fire.IA_Fire"))
  (bind _shoot_zone (`self.Shoot_Zone`))
  ;[0.2098 0.07771 0.2471] Nodes controling shells & Play Fire shoot & When set "Auto Fire" to true, Fire shooting is set to automatic control
  (:`Triggered`
    (if (and (not (`self.Cannon_Out_Off_Ammo`)) (not (`self.Use_Auto_Fire`)))
      (if (`self.UseMultiShot?`)
        (if (not (`self.Delay`))
          (`|SpawnActorFromClass` "/Game/cannon/Blueprints/BP_AdvancedCannonSystem_Projectile.BP_AdvancedCannonSystem_Projectile_C" (`KismetMathLibrary.MakeTransform` (`SceneComponent.K2_GetComponentLocation` _shoot_zone) (`SceneComponent.K2_GetComponentRotation` _shoot_zone)) "AlwaysSpawn" "OverrideRootScale" null null :!label _label) ; Spawn projectile
          (`GameplayStatics.SpawnSoundAttached` "/Game/cannon/Demo/EpicContent/Sounds/Cue/SC_Explosion_Cue.SC_Explosion_Cue" (`self.Mesh`) "None" (0.0 0.0 0.0) (struct) "KeepRelativeOffset" false 1.0 1.0 0.0 null null)
          (`GameplayStatics.PlayWorldCameraShake` "/Game/cannon/Blueprints/BP_Cannon_Fire_CameraShake.BP_Cannon_Fire_CameraShake_C" (`SceneComponent.K2_GetComponentLocation` (`self.Mesh`)) 0.0 800.0 1.0 true)
          (if (`self.UseMultiShot?`)
            (set `self.Delay` true)
            (`KismetSystemLibrary.Delay` 0.5)
            (set `self.Delay` false)
            (elif (`self.Use_Auto_Fire`)
              (`self.CE_Auto_Fire`))))
        (else
          (set `self.Cannon_Out_Off_Ammo` true)
          (`ActorComponent.Activate` (`self.PS_Muzzle_Front`) false :!label _label_2)
          (`ActorComponent.Activate` (`self.PS_Dust`) false)
          (if (`self.Use_replenishing_Shells`)
            (`self.CE_Replenish_Shells`))
          (`/Engine/EditorBlueprintResources/StandardMacros.CompareInt` (`self.Max_Shells`)
            (:`>`
              (set `self.Max_Shells` (- (`self.Max_Shells`) 1))
              (goto _label))
            (:`==`
              (set `self.Cannon_Out_Off_Ammo` true))))))))

(event `CE_Auto_Fire_Input`
  (bind _number_of_times_auto_fire_shooting (`self.Number of times Auto Fire shooting`))
  ;[0.2098 0.07771 0.2471] Nodes controling shells & Play Fire shoot & When set "Auto Fire" to true, Fire shooting is set to automatic control
  (`KismetSystemLibrary.K2_SetTimerDelegate` (delegate `CE_Auto_Fire_Input`) (`TimelineComponent.GetTimelineLength` (`self.Ammo_replenish_Timeline`)))
  (`KismetSystemLibrary.Delay` (`self.Auto_Fire_delay_at_start`))
  (bind _counter (`/Engine/EditorBlueprintResources/StandardMacros.Do N` _number_of_times_auto_fire_shooting)
    (:`Exit`
      (if (> _counter _number_of_times_auto_fire_shooting)
        (`KismetSystemLibrary.K2_ClearTimer` null "CE_Auto_Fire_Input")
        (`KismetSystemLibrary.K2_ClearTimer` null "CE_Auto_Fire")
        (elif (not (`self.Cannon_Out_Off_Ammo`))
          (goto _label_2))))))

(event `CE_Replenish_Shells`
  (bind _cannon_reload (`self.Cannon_Reload`))
  ;[0.1842 0.09188 0.2471] Nodes controling  replenishing ammo of main gun  ( every 10 seconds one shell will be added to the clip )
  ;;[1 0.1583 0.9096] Through (Use_replenishing_shells) you can set it to an False to stop the auto-replenishing in Auto-Fire at any time.
  (if (`self.Use_replenishing_Shells`)
    (`/Engine/EditorBlueprintResources/StandardMacros.DoOnce` false :!label _label_3
      (:`Completed`
        (`AudioComponent.Play` _cannon_reload 0.0)
        (`Timeline|Ammo_replenish_Timeline` :!via `PlayFromStart` :!label _label_4
          (:`Finished`
            (`AudioComponent.FadeOut` _cannon_reload 0.5 0.0 "Linear")
            (bind _output_get (set `self.Max_Shells` (+ (`self.Max_Shells`) 1)))
            (`/Engine/EditorBlueprintResources/StandardMacros.CompareInt` _output_get (`self.Shells_Missle_Ammo`)
              (:`==`
                (set `self.Cannon_Out_Off_Ammo` false)
                (goto _label_3 :!via `Reset`))
              (:`<`
                (goto _label_4 :!via `PlayFromStart`)))))))))

(event `Key|F`
  (params (Key :type "Key Structure"))
  ;[0.6985 0.1573 1] Nodes controling slow motion
  (:`Pressed`
    (`/Engine/EditorBlueprintResources/StandardMacros.FlipFlop`
      (:`A`
        (`GameplayStatics.SetGlobalTimeDilation` 0.25))
      (:`B`
        (`GameplayStatics.SetGlobalTimeDilation` 1.0)))))

(event `self.ReceiveBeginPlay`
  ;[0.9719 0.1985 1] Event BeginPlay
  ;;[0.9915 0.1511 1] Speed replenish ammo time set
  (`TimelineComponent.SetTimelineLength` (`self.Ammo_replenish_Timeline`) (`KismetMathLibrary.Conv_IntToDouble` (`self.Shells_Replenish_TIME`)))
  ;;[1 0.2226 0.9687] Set max shells for main gun " Normal ammunition loaded 1"
  (set `self.Max_Shells` (`self.Shells_Missle_Ammo`))
  (if (`self.Use_Auto_Fire`)
    ;;[0.8387 0.1303 1] Is True (Use Auto Fire) Play Event "CE_Auto_Fire_Input"
    (`self.CE_Auto_Fire_Input`)))

(event `self.ReceiveTick`
  (params (DeltaSeconds :type "Float (single-precision)"))
  (bind (_returnvalue_location _returnvalue_rotation) (`KismetMathLibrary.BreakTransform` (`SceneComponent.GetSocketTransform` (`self.Shoot_Zone`) "None" "RTS_World")))
  (bind _returnvalue (`KismetMathLibrary.GetForwardVector` _returnvalue_rotation))
  ;[0.06569 1 0.07899] select SHOOT ARRAY LINE
  (if (`self.UseArrayLine?`)
    (`self.ClearArrow`)
    (bind _predictresult (`GameplayStatics.Blueprint_PredictProjectilePath_Advanced` (make `PredictProjectilePathParams` :`StartLocation` _returnvalue_location :`LaunchVelocity` (* (+ _returnvalue (* _returnvalue 0.0)) 9000.0) :`bTraceWithCollision` true :`ProjectileRadius` 10.0 :`MaxSimTime` 10.0 :`TraceChannel` "ECC_Visibility" :`ObjectTypes` (`|MakeArray` "ObjectTypeQuery1" :!type "EObjectTypeQuery Enum") :`SimFrequency` 15.0 :`DrawDebugTime` 0.0)))
    (`self.UpdateArrowSpline` _predictresult)))

(event `Key|RightMouseButton`
  (params (Key :type "Key Structure"))
  (bind _returnvalue (`GameplayStatics.GetWorldDeltaSeconds`))
  (bind _returnvalue_2 (`GameplayStatics.GetWorldDeltaSeconds`))
  (bind _camera_fp (`self.Camera_FP`))
  (bind _camera_tp (`self.Camera_TP`))
  (bind _fieldofview (`CameraComponent.FieldOfView` _camera_tp))
  (bind _fieldofview_2 (`CameraComponent.FieldOfView` _camera_fp))
  ;[1 0.07146 0.7397] Nodes controling zoom of turret gun, via FOV
  (:`Pressed`
    (if (or (`ActorComponent.IsActive` (`self.Springarm_Main_Gun_FP`)) (`ActorComponent.IsActive` (`self.Springarm_Main_Gun_TP`)))
      (`/Engine/EditorBlueprintResources/StandardMacros.FlipFlop`
        (:`A`
          (set `self.Turret_zoom` true)
          (`Timeline|Timeline_0` :!label _label_5
            (:`Update`
              (if (or (`ActorComponent.IsActive` (`self.Springarm_Main_Gun_FP`)) (`ActorComponent.IsActive` (`self.Springarm_Main_Gun_TP`)))
                (`|ExecutionSequence`
                  (:`then_0`
                    (if (`self.Turret_zoom`)
                      (set `CameraComponent.FieldOfView` (`KismetMathLibrary.FInterpTo` _fieldofview_2 (`self.Turret_zoom_amount`) _returnvalue_2 16.0) _camera_fp)
                      (else
                        (set `CameraComponent.FieldOfView` (`KismetMathLibrary.FInterpTo` _fieldofview_2 90.0 _returnvalue_2 16.0) _camera_fp))))
                  (:`then_1`
                    (if (`self.Turret_zoom`)
                      (set `CameraComponent.FieldOfView` (`KismetMathLibrary.FInterpTo` _fieldofview (`self.Turret_zoom_amount`) _returnvalue 16.0) _camera_tp)
                      (else
                        (set `CameraComponent.FieldOfView` (`KismetMathLibrary.FInterpTo` _fieldofview 90.0 _returnvalue 16.0) _camera_tp)))))))))
        (:`B`
          (set `self.Turret_zoom` false)
          (goto _label_5 :!via `Reverse`))))))

(event `EnhancedInput|/Game/FirstPerson/Input/Actions/IA_Look`
  (params (ActionValue :type "Vector2D Structure") (ElapsedSeconds :type "Float (double-precision)") (TriggeredSeconds :type "Float (double-precision)") (InputAction :type "InputAction Object Reference" :default "/Game/FirstPerson/Input/Actions/IA_Look.IA_Look"))
  (bind _cannon_rotation (`self.Cannon_Rotation`))
  (bind (_returnvalue_roll _returnvalue_pitch) (`KismetMathLibrary.BreakRotator` (`SceneComponent.K2_GetComponentRotation` (`self.Inner cylinder for rotation`))))
  ;[0.8853 0.2417 1] Camera Input - Mouse
  (:`Triggered`
    (`|ExecutionSequence`
      (:`then_0`
        ;[1 0 0.8995] Nodes controling turret pitch and rotation
        ;;[0.8853 0.2417 1] MOVE SHOOT Above And Under
        (set `self.Connon Rot Pitch` (`KismetMathLibrary.FClamp` (+ (`self.Connon Rot Pitch`) (* (* ActionValue_Y 50.0 (`GameplayStatics.GetWorldDeltaSeconds`)) (`self.Turret_speed`))) -20.0 25.0))
        (`SceneComponent.K2_SetRelativeRotation` (`self.The_barrel_of_the_cannon_StaticMesh_2`) (`KismetMathLibrary.MakeRotator` (`self.Connon Rot Pitch`) (.yaw (`SceneComponent.RelativeRotation` (`self.The_barrel_of_the_cannon_StaticMesh_2`))) (.pitch (`SceneComponent.RelativeRotation` (`self.The_barrel_of_the_cannon_StaticMesh_2`)))) false false))
      (:`then_1`
        ;;[1 0.07192 0.768] MOVE SHOOT RIGHT /LEFT
        (if (not (`self.Disable Rotation Shoot Right /Left`))
          (bind _output_get (set `self.TargetRotation` (`KismetMathLibrary.MakeRotator` _returnvalue_roll _returnvalue_pitch (* ActionValue_X (`self.Turret_speed`)))))
          (`SceneComponent.K2_AddLocalRotation` (`self.Inner cylinder for rotation`) _output_get false false)
          ;;;[1 0 0.7748] Play sound when turret is rotating
          (if (>= (`KismetMathLibrary.Abs` ActionValue_X) 0.5)
            (`/Engine/EditorBlueprintResources/StandardMacros.DoOnce` false :!label _label_6
              (:`Completed`
                (`AudioComponent.Play` _cannon_rotation 0.0)))
            (else
              (`AudioComponent.FadeOut` _cannon_rotation 0.2 0.0 "Linear")
              (goto _label_6 :!via `Reset`))))))))

(event `self.ReceivePossessed`
  (params (NewController :type "Controller Object Reference"))
  ;[0.9639 0.0588 1] Nodes controling start
  (if (`self.Use_AdvancedCannonSystem`)
    (`|ExecutionSequence`
      (:`then_0`
        (`/Engine/EditorBlueprintResources/StandardMacros.DoOnce` false :!label _label_7
          (:`Completed`
            (`self.DisableInput` null)
            (`KismetSystemLibrary.Delay` 0.2)
            (`AudioComponent.Play` (`self.Cannon_Enter`) 0.0)
            (`KismetSystemLibrary.Delay` 0.3)
            (`self.EnableInput` null))))
      (:`then_1`
        (`PlayerCameraManager.StartCameraFade` :`self` (`GameplayStatics.GetPlayerCameraManager` 0) :`FromAlpha` 1.0 :`Duration` 0.5) ; Connect to enable camera fade in when entering vehicle
        ;;[1 0.07573 0.8464] Add hud
        (`KismetSystemLibrary.Delay` 0.1)
        (bind _returnvalue (`|CreateWidget` "/Game/cannon/Blueprints/WBP_HUD_AdvancedCannonSystem.WBP_HUD_AdvancedCannonSystem_C"))
        (bind _output_get (set `self.UMG_HUD_widget` _returnvalue))
        (`UserWidget.AddToViewport` _output_get 0)))))

(event `EnhancedInput|/Game/cannon/Demo/EpicContent/Input/Actions/IA_Use`
  (params (ActionValue :type "Vector2D Structure") (ElapsedSeconds :type "Float (double-precision)") (TriggeredSeconds :type "Float (double-precision)") (InputAction :type "InputAction Object Reference" :default "/Game/cannon/Demo/EpicContent/Input/Actions/IA_Use.IA_Use"))
  ;[0.9639 0.0588 1] Nodes controling start
  (:`Triggered`
    (goto _label_7 :!via `Reset`)))

(event `EnhancedInput|/Game/cannon/Demo/EpicContent/Input/Actions/IA_Use`
  (params (ActionValue :type "Vector2D Structure") (ElapsedSeconds :type "Float (double-precision)") (TriggeredSeconds :type "Float (double-precision)") (InputAction :type "InputAction Object Reference" :default "/Game/cannon/Demo/EpicContent/Input/Actions/IA_Use.IA_Use"))
  (bind _returnvalue (`GameplayStatics.GetPlayerController` 0))
  (bind _cannon_enter (`self.Cannon_Enter`))
  (bind _character (`self.Character`))
  (bind _umg_hud_widget (`self.UMG_HUD_widget`))
  ;[1 0 0.5541] Nodes controling exiting vehicle and reposes character
  (:`Completed`
    (`CameraComponent.SetFieldOfView` (`self.Camera_FP`) 90.0)
    (set `self.Use_AdvancedCannonSystem` false)
    (set `/Game/cannon/Blueprints/AC_AdvancedCannonSystem_Enter.bUse_BP_AdvancedCannonSystem` false (`self.GetComponentByClass` (stale `self.TR_Enter_Stationary.OnComponentBeginOverlap` OtherActor) "/Game/cannon/Blueprints/AC_AdvancedCannonSystem_Enter.AC_AdvancedCannonSystem_Enter_C"))
    (`self.K2_SetActorTransform` _character (`KismetMathLibrary.MakeTransform` (.location (`SceneComponent.K2_GetComponentToWorld` (`self.Arrow`))) (`KismetMathLibrary.MakeRotator` 0.0 0.0 (.yaw (.rotation (`SceneComponent.K2_GetComponentToWorld` (`self.Arrow`)))))) false true)
    (`self.SetActorHiddenInGame` _character false)
    (`self.SetActorEnableCollision` _character true)
    (`Controller.Possess` _returnvalue (`self.Character`))
    (`WidgetBlueprintLibrary.SetInputMode_GameOnly` _returnvalue)
    (`AudioComponent.FadeOut` (`self.Cannon_Reload`) 0.25 0.0 "Linear")
    (`AudioComponent.FadeOut` (`self.Cannon_Rotation`) 0.25 0.0 "Linear")
    (`AudioComponent.FadeOut` (`self.Cannon_Enter`) 0.25 0.0 "Linear")
    (if (`KismetSystemLibrary.IsValid` _umg_hud_widget)
      (`Widget.RemoveFromParent` _umg_hud_widget))
    (`GameplayStatics.SpawnSoundAttached` "/Game/cannon/Demo/EpicContent/Sounds/Cue/SC_VR_ungrab_Cue.SC_VR_ungrab_Cue" (`self.Mesh`) "None" (0.0 0.0 0.0) (struct) "KeepRelativeOffset" false 1.0 1.0 0.0 "/Game/cannon/Sounds/SATT_Large.SATT_Large" null)
    (`self.SetActorEnableCollision` _character true)
    (`ActorComponent.SetActive` (`self.Springarm_Main_Gun_FP`) true false)
    (`ActorComponent.SetActive` (`self.Camera_FP`) true false)
    (`KismetSystemLibrary.Delay` 0.2)
    (if (`AudioComponent.IsPlaying` _cannon_enter)
      (`AudioComponent.Stop` _cannon_enter))))

(event `self.TR_Enter_Stationary.OnComponentBeginOverlap`
  (params (OverlappedComponent :type "PrimitiveComponent Object Reference") (OtherActor :type "Actor Object Reference") (OtherComp :type "PrimitiveComponent Object Reference") (OtherBodyIndex :type Integer) (bFromSweep :type Boolean) (SweepResult :type "HitResult Structure (by ref)"))
  (bind _returnvalue (`self.GetComponentByClass` OtherActor "/Game/cannon/Blueprints/AC_AdvancedCannonSystem_Enter.AC_AdvancedCannonSystem_Enter_C"))
  ;[1 0 0.5541] Nodes controling exiting vehicle and reposes character
  (if (not (`self.Use_Auto_Fire`))
    (set `/Game/cannon/Blueprints/AC_AdvancedCannonSystem_Enter.BP_AdvancedCannonSystem` self _returnvalue)
    (set `/Game/cannon/Blueprints/AC_AdvancedCannonSystem_Enter.bNear_BP_AdvancedCannonSystem_?` true _returnvalue)
    (`/Game/cannon/Blueprints/AC_AdvancedCannonSystem_Enter.Display_text` _returnvalue)))

(event `self.TR_Enter_Stationary.OnComponentEndOverlap`
  (params (OverlappedComponent :type "PrimitiveComponent Object Reference") (OtherActor :type "Actor Object Reference") (OtherComp :type "PrimitiveComponent Object Reference") (OtherBodyIndex :type Integer))
  (bind _returnvalue (`self.GetComponentByClass` OtherActor "/Game/cannon/Blueprints/AC_AdvancedCannonSystem_Enter.AC_AdvancedCannonSystem_Enter_C"))
  ;[1 0 0.5541] Nodes controling exiting vehicle and reposes character
  (if (not (`self.Use_Auto_Fire`))
    (set `/Game/cannon/Blueprints/AC_AdvancedCannonSystem_Enter.BP_AdvancedCannonSystem` self _returnvalue)
    (set `/Game/cannon/Blueprints/AC_AdvancedCannonSystem_Enter.bNear_BP_AdvancedCannonSystem_?` false _returnvalue)
    (`/Game/cannon/Blueprints/AC_AdvancedCannonSystem_Enter.Display_text` _returnvalue)))

(fn `ClearArrow`
  (bind _spline_meshes (`self.Spline Meshes`))
  (`ActorComponent.K2_DestroyComponent` _spline_meshes)
  (`KismetArrayLibrary.Array_Clear` _spline_meshes)
  (`SplineComponent.ClearSplinePoints` (`self.ArrowPathSpline`) true))

(fn `UpdateArrowSpline`
  (params (PredictProjectilePathResult :type "PredictProjectilePathResult Structure (by ref)"))
  (bind _pathdata (break `PredictProjectilePathResult` PredictProjectilePathResult))
  (bind _arrowpathspline (`self.ArrowPathSpline`))
  (bind _arrowpathspline_2 (`self.ArrowPathSpline`))
  (bind _returnvalue (`KismetArrayLibrary.Array_LastIndex` _pathdata))
  (for _array_element _pathdata
    (`SplineComponent.AddSplinePoint` _arrowpathspline_2 (`.Location` (break `PredictProjectilePathPointData` _array_element)) "Local" true)
    (`SceneComponent.K2_SetWorldLocation` (`self.ArrowEndSphere`) (`self.FinalArrowLocation`) false false))
  (`SplineComponent.SetSplinePointType` _arrowpathspline_2 _returnvalue "CurveClamped" true)
  (set `self.FinalArrowLocation` (`.Location` (break `PredictProjectilePathPointData` (`|GetArrayItem` _pathdata _returnvalue))))
  (for _index (range (+ (- (`SplineComponent.GetNumberOfSplinePoints` (`self.ArrowPathSpline`)) 2) 1))
    (bind _returnvalue_2 (`AddComponent|NODE_AddSplineMeshComponent-0` :`bManualAttachment` true))
    (`PrimitiveComponent.SetMaterial` _returnvalue_2 1 (`self.LaserPointerMaterial`))
    (`KismetArrayLibrary.Array_Add` (`self.Spline Meshes`) _returnvalue_2)
    (bind (_location _tangent) (`SplineComponent.GetLocationAndTangentAtSplinePoint` _arrowpathspline _index "Local"))
    (bind (_location_2 _tangent_2) (`SplineComponent.GetLocationAndTangentAtSplinePoint` _arrowpathspline (+ _index 1) "Local"))
    (`SplineMeshComponent.SetStartAndEnd` _returnvalue_2 _location _tangent _location_2 _tangent_2 true)))

(fn `UserConstructionScript`
  (bind _arrowendsphere (`self.ArrowEndSphere`))
  (`|ExecutionSequence`
    (:`then_0`
      (if (`self.Switch Between Camera`)
        ;[0.7753 0.1284 1] Switch Between Third Person And First Person Camera
        (`ActorComponent.SetAutoActivate` (`self.Camera_FP`) true)
        (`ActorComponent.SetAutoActivate` (`self.Camera_TP`) false)
        (else
          (`ActorComponent.SetAutoActivate` (`self.Camera_TP`) true)
          (`ActorComponent.SetAutoActivate` (`self.Camera_FP`) false))))
    (:`then_1`
      ;[0.7313 0.1624 1] Use Target Indicator Material
      (switch `int` (`self.UseTargetIndicatorMaterial`)
        (:`Default`
          (`PrimitiveComponent.CreateDynamicMaterialInstance` _arrowendsphere 0 "/Game/cannon/Demo/EpicContent/Geometry/Materials/M_LaserPointer-Core.M_LaserPointer-Core" "None" :!label _label))
        (:`1`
          (goto _label))
        (:`2`
          (`PrimitiveComponent.CreateDynamicMaterialInstance` _arrowendsphere 0 "/Game/cannon/Demo/EpicContent/Geometry/Materials/MI_LaserPointer-Outer.MI_LaserPointer-Outer" "None"))
        (:`3`
          (`PrimitiveComponent.CreateDynamicMaterialInstance` _arrowendsphere 0 "/Game/cannon/Demo/EpicContent/Geometry/Materials/M_LaserPointer-Outer.M_LaserPointer-Outer" "None"))
        (:`4`
          (`PrimitiveComponent.CreateDynamicMaterialInstance` _arrowendsphere 0 "/Game/cannon/Demo/EpicContent/Geometry/Materials/M_LaserPointerMaterial.M_LaserPointerMaterial" "None"))
        (:`5`
          (`PrimitiveComponent.CreateDynamicMaterialInstance` _arrowendsphere 0 "/Game/cannon/Demo/EpicContent/Geometry/Materials/MI_LaserPointer.MI_LaserPointer" "None"))
        (:`6`
          (`PrimitiveComponent.CreateDynamicMaterialInstance` _arrowendsphere 0 "/Game/cannon/Demo/EpicContent/Geometry/Materials/MI_LaserPointerMaterial.MI_LaserPointerMaterial" "None"))))))