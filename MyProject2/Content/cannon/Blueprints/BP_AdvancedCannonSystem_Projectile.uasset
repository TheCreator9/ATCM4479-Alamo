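; Rocket projectile for the advanced cannon system that damages what it hits and explodes.
; On spawn it ignores its instigator, attaches a smoke trail actor and self-destructs with an explosion after a configurable delay.
; A once-only hit applies damage, fires a radial impulse, plays impact effects, sound and camera shake, and briefly shows the first player's hit marker on tagged targets, then cleans up trail and projectile.
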(event `self.ReceiveBeginPlay`
  (`PrimitiveComponent.IgnoreActorWhenMoving` (`self.CollisionComponent`) (`self.GetInstigator`) true)
  (`PrimitiveComponent.IgnoreActorWhenMoving` (`self.StaticMesh`) (`self.GetInstigator`) true)
  ;[1 0.1264 0.9877] Spawn rocket smoke
  (bind _returnvalue (`|SpawnActorFromClass` "/Game/cannon/Blueprints/BP_Rocket_Trail.BP_Rocket_Trail_C" (`KismetMathLibrary.MakeTransform` (0.0 0.0 0.0) (struct) (2.0 2.0 2.0)) "Undefined" "OverrideRootScale" null null))
  (bind _output_get (set `self.BP_Rocket_Trail` _returnvalue))
  (`self.K2_AttachToActor` _output_get self "None" "SnapToTarget" "SnapToTarget" "SnapToTarget" true)
  ;[1 0.1593 0.9455] Set Initial Speed And Destroy Missle
  (`PrimitiveComponent.IgnoreActorWhenMoving` (`self.CollisionComponent`) (`self.GetInstigator`) true)
  ;;[1 0.1645 0.9183] Destroy_missle_after_some_time ( default 10 seconds )
  (set `self.Current_speed` (`ProjectileMovementComponent.InitialSpeed` (`self.Projectile`)))
  (`KismetSystemLibrary.Delay` (`self.Delay_to_destroy_missle_after_launch`))
  (bind _output_get_2 (set `self.Initial_location` (`SceneComponent.K2_GetComponentLocation` (`self.StaticMesh`))))
  (`GameplayStatics.SpawnEmitterAtLocation` "/Game/cannon/Demo/EpicContent/Particles/PS_Generic_Explosion.PS_Generic_Explosion" _output_get_2)
  (if (`KismetSystemLibrary.IsValid` self)
    (`self.K2_DestroyActor`)))

(event `self.ReceiveHit`
  (params (MyComp :type "PrimitiveComponent Object Reference") (Other :type "Actor Object Reference") (OtherComp :type "PrimitiveComponent Object Reference") (bSelfMoved :type Boolean) (HitLocation :type "Vector Structure") (HitNormal :type "Vector Structure") (NormalImpulse :type "Vector Structure") (Hit :type "HitResult Structure (by ref)"))
  (bind (_bblockinghit _binitialoverlap _time _distance _location _impactpoint _normal _impactnormal _physmat _hitactor _hitcomponent _hitbonename _bonename _hititem _elementindex _faceindex _tracestart) (`GameplayStatics.BreakHitResult` Hit))
  (bind _returnvalue (`GameplayStatics.GetPlayerController` 0))
  (bind _bp_rocket_trail (`self.BP_Rocket_Trail`))
  ;[1 0.2791 0.9115] Spawn_sound_and_particle_on_impact
  (`/Engine/EditorBlueprintResources/StandardMacros.DoOnce` false
    (:`Completed`
      (`/Engine/EditorBlueprintResources/StandardMacros.IsValid` Other
        (:`Is Valid`
          (`GameplayStatics.ApplyDamage` Other 100.0 null (`self.GetInstigator`)))
        (:`Is Not Valid`
          _))
      (`/Engine/EditorBlueprintResources/StandardMacros.DoOnce` false
        (:`Completed`
          (`RadialForceComponent.FireImpulse` (`self.RadialForce1`))
          (`GameplayStatics.SpawnEmitterAtLocation` (`self.PS_Impact_Emmiter`) HitLocation (`KismetMathLibrary.MakeRotator` (.x _tracestart) (.y _tracestart))) ; Spawn impact emmiter
          (`GameplayStatics.PlayWorldCameraShake` "/Game/cannon/Blueprints/BP_Impact_HI_Explosive_CameraShake.BP_Impact_HI_Explosive_CameraShake_C" HitLocation 0.0 1250.0 1.0 true) ; Spawn camera shake at impact
          (`/Engine/EditorBlueprintResources/StandardMacros.IsValid` Other
            (:`Is Valid`
              (if (and _bblockinghit (== (`self.GetInstigatorController`) (`GameplayStatics.GetPlayerController` 0)) (`self.ActorHasTag` _hitactor "HitMarker"))
                (bind _returnvalue_2 (`|CreateWidget` "/Game/cannon/Blueprints/WBP_Hit_Marker.WBP_Hit_Marker_C" _returnvalue))
                (bind _output_get (set `self.UMG_Hit_Marker` _returnvalue_2))
                (`UserWidget.SetPositionInViewport` _output_get (`WidgetLayoutLibrary.ProjectWorldLocationToWidgetPosition` _returnvalue HitLocation) false)
                (`UserWidget.AddToViewport` _output_get 0)
                (`KismetSystemLibrary.Delay` 0.1)
                (`Widget.RemoveFromParent` _output_get)))
            (:`Is Not Valid`
              _))
          (`GameplayStatics.PlaySoundAtLocation` "/Game/cannon/Demo/EpicContent/Sounds/Cue/SC_Explosive_Weapon_Impact_Generic.SC_Explosive_Weapon_Impact_Generic" (`SceneComponent.K2_GetComponentLocation` (`self.StaticMesh`)) (struct) 1.0 1.0 0.0 null null null null)
          (`ActorComponent.Deactivate` (`Actor.RootComponent` _bp_rocket_trail))
          (`KismetSystemLibrary.Delay` 0.3)
          (`SceneComponent.SetVisibility` (`self.StaticMesh`) false false)
          (`PrimitiveComponent.SetCollisionEnabled` (`self.CollisionComponent`) "NoCollision")
          (`PrimitiveComponent.SetCollisionEnabled` (`self.StaticMesh`) "NoCollision")
          (`KismetSystemLibrary.Delay` 0.1)
          (`/Engine/EditorBlueprintResources/StandardMacros.IsValid` _bp_rocket_trail
            (:`Is Valid`
              (`self.K2_DestroyActor` _bp_rocket_trail))
            (:`Is Not Valid`
              _))
          (if (`KismetSystemLibrary.IsValid` self)
            (`self.K2_DestroyActor`)))))))

(fn `UserConstructionScript`
  (`SphereComponent.SetSphereRadius` (`self.VIS_Explosion_Radius`) (`self.Explosion_Radius`) true))