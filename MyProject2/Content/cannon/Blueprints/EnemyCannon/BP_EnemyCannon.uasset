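; BP_EnemyCannon is an enemy cannon built from static mesh parts that is wrecked the first time it takes any damage.
; A DoOnce on AnyDamage spawns BP_EnemyCannon_Destroyed at the cannon's transform, flags it as destroyed and calls its CEDestroyWreck event.
; The intact cart, barrel, wheels and wedge lose collision and visibility, then the actor destroys itself after a short delay.
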(event `self.ReceiveAnyDamage`
  (params (Damage :type "Float (single-precision)") (DamageType :type "DamageType Object Reference") (InstigatedBy :type "Controller Object Reference") (DamageCauser :type "Actor Object Reference"))
  (bind _wedge_staticmesh_3 (`self.wedge_StaticMesh_3`))
  ;[0.9334 0.1473 1] damage system
  (`/Engine/EditorBlueprintResources/StandardMacros.DoOnce` false
    (:`Completed`
      (bind _returnvalue (`|SpawnActorFromClass` "/Game/cannon/Blueprints/EnemyCannon/BP_EnemyCannon_Destroyed.BP_EnemyCannon_Destroyed_C" (`self.GetTransform`) "Undefined" "OverrideRootScale" null null))
      (set `/Game/cannon/Blueprints/EnemyCannon/BP_EnemyCannon_Destroyed.Wreck_destroyed_?` true _returnvalue)
      (`/Game/cannon/Blueprints/EnemyCannon/BP_EnemyCannon_Destroyed.CE_Destroy_Wreck` _returnvalue)
      (`PrimitiveComponent.SetCollisionEnabled` _wedge_staticmesh_3 "NoCollision")
      (`PrimitiveComponent.SetCollisionEnabled` (`self.Left_rear_wheel_StaticMesh_7`) "NoCollision")
      (`PrimitiveComponent.SetCollisionEnabled` (`self.Right_rear_wheel_StaticMesh_6`) "NoCollision")
      (`PrimitiveComponent.SetCollisionEnabled` (`self.Cannon_cart_StaticMesh_1`) "NoCollision")
      (`PrimitiveComponent.SetCollisionEnabled` (`self.Right_front_wheel_StaticMesh_4`) "NoCollision")
      (`PrimitiveComponent.SetCollisionEnabled` (`self.The_barrel_of_the_cannon_StaticMesh_2`) "NoCollision")
      (`PrimitiveComponent.SetCollisionEnabled` (`self.left_front_wheel_StaticMesh_5`) "NoCollision")
      (`SceneComponent.SetVisibility` _wedge_staticmesh_3 false false)
      (`SceneComponent.SetVisibility` (`self.Left_rear_wheel_StaticMesh_7`) false false)
      (`SceneComponent.SetVisibility` (`self.Right_rear_wheel_StaticMesh_6`) false false)
      (`SceneComponent.SetVisibility` (`self.Cannon_cart_StaticMesh_1`) false false)
      (`SceneComponent.SetVisibility` (`self.Right_front_wheel_StaticMesh_4`) false false)
      (`SceneComponent.SetVisibility` (`self.The_barrel_of_the_cannon_StaticMesh_2`) false false)
      (`SceneComponent.SetVisibility` (`self.left_front_wheel_StaticMesh_5`) false false)
      (`KismetSystemLibrary.Delay` 0.1)
      (`self.K2_DestroyActor`))))

(fn `UserConstructionScript`)