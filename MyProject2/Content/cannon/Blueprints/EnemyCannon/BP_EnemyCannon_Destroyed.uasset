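; BP_EnemyCannon_Destroyed is the wreck of a destroyed enemy cannon, with explosion, fire and sound effects.
; On BeginPlay or the destroy-wreck event, a WreckDestroyed check and a DoOnce gate a one-time sequence.
; It spawns an attached explosion emitter and activates the turret particles and burning-fire sound.
; After a fixed delay it fades out the sound and deactivates both hull and turret particles.
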(event `CE_Destroy_Wreck`
  (bind _cs_fire_burning (`self.CS_Fire_burning`))
  ;[0.9769 0.2077 1] Destroy Wreck
  (if (`self.Wreck_destroyed_?`) :!label _label
    (`/Engine/EditorBlueprintResources/StandardMacros.DoOnce` false
      (:`Completed`
        (`GameplayStatics.SpawnEmitterAttached` "/Game/cannon/Demo/EpicContent/Particles/PS_Generic_Explosion.PS_Generic_Explosion" null "Root")
        ;;[0.8924 0.1314 1] Play primary PS effect, and play fire and explosion sound
        (`ActorComponent.SetActive` (`self.PS_Turret`) true false)
        (`ActorComponent.SetActive` _cs_fire_burning true false)
        (`KismetSystemLibrary.Delay` 19.0) ; Change this to control how long PS effect will be played
        (`AudioComponent.FadeOut` _cs_fire_burning 2.0 0.0 "Linear")
        (`ActorComponent.SetActive` (`self.PS_Hull`) false false)
        (`ActorComponent.SetActive` (`self.PS_Turret`) false false)))))

(event `self.ReceiveBeginPlay`
  ;[0.9769 0.2077 1] Destroy Wreck
  (goto _label))

(fn `UserConstructionScript`)